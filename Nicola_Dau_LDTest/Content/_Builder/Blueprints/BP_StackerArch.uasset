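; BP_StackerArch is a builder actor that places copies of a chosen mesh along a circular arc.
; When Generate is set, its construction script fills an InstancedStaticMesh, with Mode deriving count and angular step from amount, angle or arch span.
; Per-index location, rotation and scale offsets accumulate along the arc, allowing rising or tapering stacks.
; Options control arc centering and whether instance yaw follows the arc angle.
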(event EventBeginPlay)

(event Collision|EventActorBeginOverlap
  (params (OtherActor :type Actor%20Object%20Reference)))

(event EventTick
  (params (DeltaSeconds :type Float%20%28single-precision%29)))

(fn ConstructionScript
  (bind _angle (Variables|Details|GetAngle))
  (bind _locationbase (Variables|Extra|GetLocationBase))
  (bind _archangle (Variables|Details|GetArchAngle))
  (bind _angle_2 (Variables|Details|GetAngle))
  (if (Variables|Base|GetGenerate)
    (Components|StaticMesh|SetStaticMesh (Variables|Default|GetInstancedStaticMesh) (Variables|Base|GetMesh))
    (for _index (range 0 (Utilities|Select :Index (Variables|Base|GetMode) :NewEnumerator0 (- (Variables|Details|GetAmount) 1) :NewEnumerator1 (- (Variables|Details|GetAmount) 1) :NewEnumerator2 (Math|Float|Floor (/ _archangle (Math|Float|SelectFloat _archangle _angle_2 (== _angle_2 0.0))))))
      (Components|InstancedStaticMesh|AddInstance (Variables|Default|GetInstancedStaticMesh) (Math|Transform|MakeTransform (+ (Math|Vector|SelectVector _locationbase (+ (Math|Vector|MakeVector 0.0 (* (Variables|Base|GetRadius) -1.0) 0.0) _locationbase) (Variables|Base|GetCenter)) (* (Math|Vector|MakeVector (Math|Trig|Cos(Degrees) (+ (Variables|Base|GetBaseAngle) (* _index (Utilities|Select :Index (Variables|Base|GetMode) :NewEnumerator0 _angle :NewEnumerator1 (/ (Variables|Details|GetArchAngle) (Math|Conversions|ToFloat(Integer) (Math|Integer|Max(Integer) (Variables|Details|GetAmount) 1))) :NewEnumerator2 _angle)))) (Math|Trig|Sin(Degrees) (+ (Variables|Base|GetBaseAngle) (* _index (Utilities|Select :Index (Variables|Base|GetMode) :NewEnumerator0 _angle :NewEnumerator1 (/ (Variables|Details|GetArchAngle) (Math|Conversions|ToFloat(Integer) (Math|Integer|Max(Integer) (Variables|Details|GetAmount) 1))) :NewEnumerator2 _angle)))) 0.0) (Variables|Base|GetRadius)) (* (Variables|Extra|GetLocationOffset) _index)) (Math|Rotator|CombineRotators (Math|Rotator|SelectRotator (Math|Rotator|MakeRotator 0.0 0.0 (+ (Variables|Base|GetBaseAngle) (* _index (Utilities|Select :Index (Variables|Base|GetMode) :NewEnumerator0 _angle :NewEnumerator1 (/ (Variables|Details|GetArchAngle) (Math|Conversions|ToFloat(Integer) (Math|Integer|Max(Integer) (Variables|Details|GetAmount) 1))) :NewEnumerator2 _angle)))) (* (Variables|Extra|GetRotationOffset) _index) (Variables|Extra|GetFaceCenter)) (Variables|Extra|GetRotationBase)) (+ (* (Variables|Extra|GetScaleOffset) _index) (Variables|Extra|GetScaleBase)))))))