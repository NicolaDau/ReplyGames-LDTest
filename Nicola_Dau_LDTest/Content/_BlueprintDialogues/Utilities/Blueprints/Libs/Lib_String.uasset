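; String function library in the dialogue utilities, extending the built-in parse, split, find and replace operations with escape support.
; FindSubstring2 skips escaped matches, using a recursive check for escaped escapes, and underpins Split2, ParseIntoArray2 and ExtractTextBetweenCharacters, which can match nested pairs.
; ParseIntoArray2 can keep delimiters, falling back to the built-in version when possible.
; Other helpers parse trailing numbers, list substring positions, replace by index and strip single-character escapes.
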(fn ParseTrailingNumberfromString
  (params (Text :type String))
  (Utilities|FlowControl|Sequence
    (:then_0
      ;[1 1 1] Extract trailing numbers
      (bind _output_get (LocalVariables|SetReverseCharacters (Utilities|String|GetCharacterArrayfromString (Utilities|String|Reverse Text))))
      (bind _array_element (Utilities|Array|ForEachLoopwithBreak _output_get :!label _label)
        (:LoopBody
          (if (Class|KismetStringLibrary|IsNumeric _array_element)
            (Utilities|Array|Insert (LocalVariables|GetTrailingNumberCharacters) _array_element)
            (else
              (goto _label Break))))))
    (:then_1
      ;[1 1 1] Extract text before number
      (LocalVariables|SetTextBeforeNumber (Utilities|String|GetSubstring Text 0 (- (Utilities|String|Len Text) (Utilities|Array|Length (LocalVariables|GetTrailingNumberCharacters))))))
    (:then_2
      ;[1 1 1] Recombine the number into a string
      (for _array_element_2 (LocalVariables|GetTrailingNumberCharacters)
        (LocalVariables|SetDigitString (Utilities|String|Append (LocalVariables|GetDigitString) _array_element_2))))
    (:then_3
      (return (Math|Conversions|ToInteger(Byte) (LocalVariables|GetDigitString)) (LocalVariables|GetTextBeforeNumber)))))

(fn ExtractTextBetweenCharacters
  (params (Text :type String) (StartingText :type String) (EndingText :type String) (StartPosition :type Integer) (Use%20Case :type Boolean) (EscapeString :type String) (Paired :type Boolean))
  (Utilities|FlowControl|Sequence
    (:then_0
      (Utilities|FlowControl|Sequence
        (:then_0
          (LocalVariables|SetStartTextSub StartingText))
        (:then_1
          (LocalVariables|SetEndingTextSub EndingText))
        (:then_2
          (LocalVariables|SetCaseSensitive Use%20Case))
        (:then_3
          (LocalVariables|SetEscapeSubString EscapeString))))
    (:then_1
      (if (< StartPosition (Utilities|String|Len Text))
        (Utilities|FlowControl|Sequence
          (:then_0
            (bind _return_value (Utilities|String|FindSubstring2 Text (LocalVariables|GetStartTextSub) (LocalVariables|GetCaseSensitive) false StartPosition (LocalVariables|GetEscapeSubString))) ; Find first instance of start
            (bind _output_get (LocalVariables|SetsubStart _return_value))
            (if (>= _output_get 0)
              (if Paired
                (|FindMatchingPairEnd Text)
                (else
                  (bind _return_value_2 (Utilities|String|FindSubstring2 Text (LocalVariables|GetEndingTextSub) (LocalVariables|GetCaseSensitive) false (+ (LocalVariables|GetsubStart) (Utilities|String|Len (LocalVariables|GetStartTextSub))) (LocalVariables|GetEscapeSubString))) ; Find first instance of end - ignore pairings
                  (LocalVariables|SetsubEnd _return_value_2)))))
          (:then_1
            ;[1 1 1] Extract Text
            (if (and (>= (LocalVariables|GetsubStart) 0) (>= (LocalVariables|GetsubEnd) 0))
              (bind _output_get_2 (LocalVariables|SetFound (Utilities|String|GetSubstring Text (LocalVariables|GetsubStart) (+ (- (LocalVariables|GetsubEnd) (LocalVariables|GetsubStart)) 1))))
              (if (> (Utilities|String|Len _output_get_2) 1)
                (LocalVariables|SetInBetweenText (Utilities|String|GetSubstring _output_get_2 1 (- (Utilities|String|Len _output_get_2) 2)))
                (else
                  (LocalVariables|SetInBetweenText _output_get_2)))))
          (:then_2
            (return (LocalVariables|GetFound) (LocalVariables|GetInBetweenText) (LocalVariables|GetsubStart) (LocalVariables|GetsubEnd))))
        (else
          (return (LocalVariables|GetFound) (LocalVariables|GetInBetweenText) (LocalVariables|GetsubStart) (LocalVariables|GetsubEnd)))))))

(fn ParseIntoArray2
  (params (SourceString :type String) (Delimiter :type String) (CullEmptyStrings :type Boolean) (PreserveDelimiter :type Boolean) (EscapeString :type String))
  (Utilities|FlowControl|Sequence
    (:then_0
      (if (|ValidStringanddelimiter SourceString Delimiter)
        (if (or PreserveDelimiter (> (Utilities|String|Len (Utilities|String|Trim EscapeString)) 0))
          (|ConfigureVariables SourceString Delimiter)
          (Utilities|DoWhilewithBreak (and (>= (LocalVariables|GetNewFoundIdx) 0) (< (LocalVariables|GetNewFoundIdx) (- (LocalVariables|GetSourceLength) 1)))
            (:Loop%20Body
              (bind _return_value (Utilities|String|FindSubstring2 SourceString Delimiter false false (+ (LocalVariables|GetLastFoundEndIdx) 1) EscapeString))
              (bind _output_get (LocalVariables|SetNewFoundIdx _return_value))
              (bind _newdelimitedpartition (Utilities|String|GetSubstring SourceString (>= _output_get 0) PreserveDelimiter))
              (bind _output_get_2 (LocalVariables|SetNewDelimited _newdelimitedpartition))
              (LocalVariables|SetLastFoundEndIdx (+ (LocalVariables|GetDelimiterLength) (LocalVariables|GetNewFoundIdx)))
              (if (or (> (Utilities|String|Len _output_get_2) 0) (not CullEmptyStrings)) ; if( not CullEmpty or NotEmpty)
                (Utilities|Array|Add (LocalVariables|GetDelimitedStrings) (LocalVariables|GetNewDelimited)))))
          (else
            ;[1 1 1] Use built in version if possible
            (LocalVariables|SetDelimitedStrings (Utilities|String|ParseIntoArray SourceString Delimiter CullEmptyStrings))))))
    (:then_1
      (return (LocalVariables|GetDelimitedStrings)))))

(fn FindAllSubstringPositions
  (params (SearchIn :type String) (Substring :type String) (UseCase :type Boolean) (StartPosition :type Integer))
  (bind _returnvalue (Utilities|String|Len Substring))
  (Utilities|FlowControl|Sequence
    (:then_0
      (LocalVariables|SetLastFound StartPosition)
      (Utilities|FlowControl|Sequence ; do while
        (:then_0
          (bind _output_get (LocalVariables|SetLastFound (Utilities|String|FindSubstring SearchIn Substring UseCase false (LocalVariables|GetLastFound)) :!label _label))
          (if (!= _output_get -1)
            (Utilities|Array|Add (LocalVariables|GetPositions) (LocalVariables|GetLastFound))))
        (:then_1
          (while (and (< (LocalVariables|GetLastFound) (- (Utilities|String|Len SearchIn) _returnvalue)) (>= (LocalVariables|GetLastFound) 0))
            (LocalVariables|SetLastFound (+ (LocalVariables|GetLastFound) _returnvalue))
            (goto _label)))))
    (:then_1
      (return (LocalVariables|GetPositions)))))

(fn FindSubstring2
  (params (SearchIn :type String) (Substring :type String) (UseCase :type Boolean) (SearchFromEnd :type Boolean) (StartPosition :type Integer) (EscapeString :type String))
  (Utilities|FlowControl|Sequence
    (:then_0
      (LocalVariables|SetLastFoundResult StartPosition)
      (Utilities|FlowControl|Sequence ; do while
        (:then_0
          _)
        (:then_1
          (Utilities|WhilewithBreak (|HasPassedEnd SearchIn Substring) :!label _label
            (:Loop%20Body
              (|IncrementPointer SearchFromEnd SearchIn Substring)))))
      (bind _output_get (LocalVariables|SetLastFoundResult (Utilities|String|FindSubstring SearchIn Substring UseCase SearchFromEnd (LocalVariables|GetLastFoundResult))))
      (bind _isescaped (Utilities|String|IsEscapedSubstring SearchIn _output_get EscapeString UseCase))
      (if _isescaped
        (bind _count (Utilities|Counter -1))
        (if (> _count 50)
          (goto _label break))
        (else
          (LocalVariables|SetFound (LocalVariables|GetLastFoundResult))
          (LocalVariables|SetLastFoundResult -1) ; Break out of loop
        )))
    (:then_1
      (return (LocalVariables|GetFound)))))

(fn IsEscapedSubstring
  (params (SourceString :type String) (StartIndex :type Integer) (EscapeString :type String) (UseCase :type Boolean))
  (bind _returnvalue (Utilities|String|Len EscapeString))
  (bind _returnvalue_2 (- StartIndex _returnvalue))
  (if (|IsEscapePossible _returnvalue_2 EscapeString)
    (Utilities|FlowControl|Sequence
      (:then_0
        (bind _result (Utilities|String|StringEqual EscapeString (Utilities|String|GetSubstring SourceString _returnvalue_2 _returnvalue) UseCase))
        (if _result
          ;[1 1 1] Make sure the escape string is not escaped
          (bind _isescaped (Utilities|String|IsEscapedSubstring SourceString _returnvalue_2 EscapeString UseCase))
          (LocalVariables|SetEscaped (not _isescaped))))
      (:then_1
        (return (LocalVariables|GetEscaped))))
    (else
      (return (LocalVariables|GetEscaped)))))

(fn StringEqual
  (params (String1 :type String) (String2 :type String) (UseCase :type Boolean))
  (Utilities|FlowControl|Sequence
    (:then_0
      (if UseCase
        (LocalVariables|SetIsEqual (Utilities|Enum|Equal(Enum) String1 String2))
        (else
          (LocalVariables|SetIsEqual (Utilities|Enum|Equal(Enum) String1 String2)))))
    (:then_1
      (return (LocalVariables|GetIsEqual)))))

(fn ReplacebyLocation
  (params (SourceString :type String) (ReplaceWith :type String) (StartReplacingLocation :type Integer) (EndReplacingLocation :type Integer))
  (bind _returnvalue (+ EndReplacingLocation 1))
  (if (<= EndReplacingLocation StartReplacingLocation)
    (LocalVariables|SetResult SourceString)
    (return (LocalVariables|GetResult))
    (else
      (Utilities|FlowControl|Sequence
        (:then_0
          (Utilities|FlowControl|Sequence
            (:then_0
              (LocalVariables|SetBefore (Utilities|String|GetSubstring SourceString 0 StartReplacingLocation)))
            (:then_1
              (LocalVariables|SetAfter (Utilities|String|GetSubstring SourceString _returnvalue (- (Utilities|String|Len SourceString) _returnvalue))))))
        (:then_1
          (LocalVariables|SetResult (Utilities|String|Append (Utilities|String|Append (LocalVariables|GetBefore) ReplaceWith) (LocalVariables|GetAfter))))
        (:then_2
          (return (LocalVariables|GetResult)))))))

(fn Split2
  (params (Source%20String :type String) (In%20Str :type String) (UseCase :type Boolean) (Search%20from%20End :type Boolean) (Escape%20String :type String) (KeepDelimiter :type Boolean))
  (bind _returnvalue (Utilities|String|Len Source%20String))
  (bind _return_value (Utilities|String|FindSubstring2 Source%20String In%20Str UseCase Search%20from%20End -1 Escape%20String))
  (if (< _return_value 0)
    (return Source%20String "" false)
    (else
      (return (Utilities|String|Left Source%20String _return_value) (select KeepDelimiter (Utilities|String|Right Source%20String (- _returnvalue _return_value)) (Class|KismetStringLibrary|Mid Source%20String (+ _return_value (Utilities|String|Len In%20Str)) (Math|Integer|Max(Integer) _returnvalue))) true))))

(fn RemoveEscapeCharacters
  (params (SourceString :type String) (EscapeCharacter :type String))
  (Utilities|FlowControl|Sequence
    (:then_0
      (if (== (Utilities|String|Len EscapeCharacter) 1)
        (bind _output_get (LocalVariables|SetInArray (Utilities|String|GetCharacterArrayfromString SourceString)))
        (for _array_element _output_get
          (if (and (Utilities|Enum|Equal(Enum) _array_element EscapeCharacter) (not (LocalVariables|GetWasLastEscapeStr)))
            (LocalVariables|SetWasLastEscapeStr true)
            (else
              (Utilities|Array|Add (LocalVariables|GetCleanedArray) _array_element)
              (LocalVariables|SetWasLastEscapeStr false))))
        (else
          (Development|PrintString 0 "RemoveEscapeCharacters only supports single character escapes" true true "(R=1.000000,G=0.000000,B=0.064280,A=1.000000)" 1e+01) ; ERROR
        )))
    (:then_1
      (return (Utilities|String|JoinStringArray (LocalVariables|GetCleanedArray) "")))))