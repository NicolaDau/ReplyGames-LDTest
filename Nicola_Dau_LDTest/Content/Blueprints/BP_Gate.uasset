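; BP_Gate is an interactable gate that opens when the player character has collected all keys.
; A Box overlap sets an in-range flag for ThirdPersonCharacter and toggles an on-screen debug-string prompt.
; Pressing E in range checks the character's AllKeys flag, then plays the Open timeline, which adds its Pos output to the actor's current location every update, so movement accumulates.
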(event OnComponentBeginOverlap(Box)
  (params (OverlappedComponent :type Primitive%20Component%20Object%20Reference) (OtherActor :type Actor%20Object%20Reference) (OtherComp :type Primitive%20Component%20Object%20Reference) (OtherBodyIndex :type Integer) (bFromSweep :type Boolean) (SweepResult :type Hit%20Result%20Structure%20%28by%20ref%29))
  ;[1 1 1] Interaction range
  (Utilities|Casting|CastToThirdPersonCharacter OtherActor)
  (Variables|Default|SetInRange true)
  (Rendering|Debug|DrawDebugString (Transformation|GetActorLocation) "Press \"E\" to Interact" 0 "(R=1.000000,G=0.025833,B=0.426000,A=1.000000)" 1e+01))

(event OnComponentEndOverlap(Box)
  (params (OverlappedComponent :type Primitive%20Component%20Object%20Reference) (OtherActor :type Actor%20Object%20Reference) (OtherComp :type Primitive%20Component%20Object%20Reference) (OtherBodyIndex :type Integer))
  ;[1 1 1] Interaction range
  (Utilities|Casting|CastToThirdPersonCharacter OtherActor)
  (Variables|Default|SetInRange false)
  (Class|KismetSystemLibrary|FlushDebugStrings))

(event EventBeginPlay
  (Input|EnableInput (Game|GetPlayerController 0)))

(event Input|KeyboardEvents|E
  (params (Key :type Key%20Structure :default "None"))
  ;[1 1 1] If the Player has all the keys, open
  (:Pressed
    (if (Variables|Default|GetInRange)
      (bind _asthird_person_character (Utilities|Casting|CastToThirdPersonCharacter (Game|GetPlayerCharacter 0)))
      (if (Variables|/Game/_StarterContent/ThirdPersonBP/Blueprints/ThirdPersonCharacter.ThirdPersonCharacter_C|GetAllKeys _asthird_person_character)
        (bind _pos (Timeline|Open Play)
          (:Update
            (Transformation|SetActorLocation (+ (Transformation|GetActorLocation) _pos) false false)))))))

(fn ConstructionScript)