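; BP_Key is a spinning key pickup that grants the player Design, Technology or Art when E is pressed in range.
; A collision overlap with the ThirdPersonCharacter toggles InRange and shows or flushes a debug-string prompt.
; On E, the first true Give flag sets the matching Has flag on the character, calls OnKeyPickup and destroys the key.
; It enables its own input on BeginPlay to receive the key press directly.
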(event OnComponentBeginOverlap(Collision)
  (params (OverlappedComponent :type Primitive%20Component%20Object%20Reference) (OtherActor :type Actor%20Object%20Reference) (OtherComp :type Primitive%20Component%20Object%20Reference) (OtherBodyIndex :type Integer) (bFromSweep :type Boolean) (SweepResult :type Hit%20Result%20Structure%20%28by%20ref%29))
  ;[1 1 1] Interaction Range
  (Utilities|Casting|CastToThirdPersonCharacter OtherActor)
  (Variables|Default|SetInRange true)
  (Rendering|Debug|DrawDebugString (Transformation|GetActorLocation) "Press \"E\" to Interact" 0 "(R=1.000000,G=0.025833,B=0.426000,A=1.000000)" 1e+01))

(event OnComponentEndOverlap(Collision)
  (params (OverlappedComponent :type Primitive%20Component%20Object%20Reference) (OtherActor :type Actor%20Object%20Reference) (OtherComp :type Primitive%20Component%20Object%20Reference) (OtherBodyIndex :type Integer))
  ;[1 1 1] Interaction Range
  (Utilities|Casting|CastToThirdPersonCharacter OtherActor)
  (Variables|Default|SetInRange false)
  (Class|KismetSystemLibrary|FlushDebugStrings))

(event EventBeginPlay
  (Input|EnableInput (Game|GetPlayerController 0)))

(event EventTick
  (params (DeltaSeconds :type Float%20%28single-precision%29))
  (Transformation|AddLocalRotation (Variables|Default|GetStaticMesh) (* (Math|Rotator|MakeRotator 0.0 0.0 1.5e+02) DeltaSeconds) false false))

(event Input|KeyboardEvents|E
  (params (Key :type Key%20Structure :default "None"))
  ;[1 1 1] Add key to player inventory
  (:Pressed
    (if (Variables|Default|GetInRange)
      (bind _asthird_person_character (Utilities|Casting|CastToThirdPersonCharacter (Game|GetPlayerCharacter 0)))
      (if (Variables|Default|GetGiveDesign)
        (Variables|/Game/_StarterContent/ThirdPersonBP/Blueprints/ThirdPersonCharacter.ThirdPersonCharacter_C|SetHasDesign _asthird_person_character true)
        (Default|OnKeyPickup _asthird_person_character :!label _label)
        (Actor|DestroyActor)
        (elif (Variables|Default|GetGiveTechnology)
          (Variables|/Game/_StarterContent/ThirdPersonBP/Blueprints/ThirdPersonCharacter.ThirdPersonCharacter_C|SetHasTechnology _asthird_person_character true)
          (goto _label)
          (elif (Variables|Default|GetGiveArt)
            (Variables|/Game/_StarterContent/ThirdPersonBP/Blueprints/ThirdPersonCharacter.ThirdPersonCharacter_C|SetHasArt _asthird_person_character true)
            (goto _label)))))))

(fn ConstructionScript)