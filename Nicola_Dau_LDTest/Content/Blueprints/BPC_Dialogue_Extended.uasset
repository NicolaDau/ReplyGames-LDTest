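; Dialogue component that extends a parent dialogue class with game-specific script commands for the third-person player.
; GetScriptInterpreter supplies the interpreter stored on the ThirdPersonGameMode.
; HandleScriptFunction matches command names to set the character's Design, Art and Tech flags, passing unknown commands to the parent handler.
; The End Level command plays the LevelEnd sequence, shows the HIRED widget and destroys the player character.
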(event EventBeginPlay)

(event EventTick
  (params (DeltaSeconds :type Float%20%28single-precision%29)))

(fn GetScriptInterpreter
  (bind _asthird_person_game_mode (Utilities|Casting|CastToThirdPersonGameMode (Game|GetGameMode)))
  (return (Variables|/Game/_StarterContent/ThirdPersonBP/Blueprints/ThirdPersonGameMode.ThirdPersonGameMode_C|GetScriptInterp _asthird_person_game_mode)))

(fn HandleScriptFunction
  (params (Function :type Name :default "None") (Args :type Array%20of%20Strings))
  (Utilities|FlowControl|Sequence
    (:then_0
      (bind _asthird_person_character (Utilities|Casting|CastToThirdPersonCharacter (Game|GetPlayerCharacter 0)))
      (switch name Function
        (:Default
          (bind _result (|CallParentFunction Function Args))
          (LocalVariables|SetReturnVal _result))
        (:GiveDesign
          (Variables|/Game/_StarterContent/ThirdPersonBP/Blueprints/ThirdPersonCharacter.ThirdPersonCharacter_C|SetHasDesign _asthird_person_character true))
        (:GiveArt
          (Variables|/Game/_StarterContent/ThirdPersonBP/Blueprints/ThirdPersonCharacter.ThirdPersonCharacter_C|SetHasArt _asthird_person_character true))
        (:GiveTech
          (Variables|/Game/_StarterContent/ThirdPersonBP/Blueprints/ThirdPersonCharacter.ThirdPersonCharacter_C|SetHasTechnology _asthird_person_character true))
        (:EndLevel
          (bind _outactor (Sequencer|Player|CreateLevelSequencePlayer "/Game/Misc/LevelEnd.LevelEnd"))
          (Sequencer|Player|Play (Variables|/Script/LevelSequence.LevelSequenceActor|GetSequencePlayer _outactor) :!class /Script/MovieScene.MovieSceneSequencePlayer)
          (bind _returnvalue (UserInterface|CreateWidget "/Game/Misc/HIRED.HIRED_C"))
          (bind _output_get (Variables|Default|SetHired _returnvalue))
          (UserInterface|Viewport|AddtoViewport _output_get 0)
          (Actor|DestroyActor (Game|GetPlayerCharacter 0)))))
    (:then_1
      (return (LocalVariables|GetReturnVal)))))